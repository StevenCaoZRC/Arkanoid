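; Game mode for an Arkanoid-style game that runs each level's ball, lives, block count and win or lose flow.
; BeginPlay attaches a new ball to the paddle's socket, counts blocks and enables power-up spawning only in Level_3.
; Tick polls counters: losing all balls costs a GameInstance life and resets ball and power-up effects.
; Zero lives opens the menu level; zero blocks pauses and shows the victory widget.
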(event EventBeginPlay
  (bind _asarkanoid_game_instance (Utilities|Casting|CastToArkanoidGameInstance (Game|GetGameInstance)))
  (Variables|Default|SetGameInstanceRef _asarkanoid_game_instance)
  (CallFunction|ResetBallandPlayer)
  ;[1 1 1] Adquires the number of blocks in the current level
  (bind _outactors (Actor|GetAllActorsOfClass "/Game/Blueprints/BP_Block.BP_Block_C"))
  (Variables|Default|SetArrayOfBlocks _outactors)
  (bind _output_get (Variables|Default|SetAmountOfBlocks (Utilities|Array|Length _outactors)))
  (Development|PrintString (Utilities|String|ToString(Integer) _output_get))
  (bind _returnvalue (Game|GetCurrentLevelName true))
  (if (Utilities|Enum|Equal(Enum) _returnvalue "Level_3")
    ;[1 1 1] Will only activate the power ups and allow them to spawn in Level 3
    (for _index (range 0 (- (Utilities|Array|Length (Variables|Default|GetArrayOfBlocks)) 1))
      (Variables|/Script/Arkanoid.Block|SetbCanSpawnPowerups (Utilities|Array|Get(acopy) (Variables|Default|GetArrayOfBlocks) _index) true)))
  (Game|SetGamePaused false)
  (Input|SetInputModeGameOnly (Game|GetPlayerController 0)))

(event EventTick
  (params (DeltaSeconds :type Float%20%28single-precision%29))
  (if (<= (Variables|Default|GetBallsInLevel) 0)
    ;[1 1 1] When Player loses a life
    (Math|Integer|DecrementInt (Variables|/Script/Arkanoid.ArkanoidGameInstance|GetPlayerLives (Variables|Default|GetGameInstanceRef))
      (:%20%20
        (CallFunction|ResetBallandPlayer)
        (Class|ArkanoidGameModeBase|RevertPowerups))))
  (if (<= (Variables|/Script/Arkanoid.ArkanoidGameInstance|GetPlayerLives (Variables|Default|GetGameInstanceRef)) 0)
    ;[1 1 1] Game Over
    (Game|OpenLevel(byName) "Level_Menu")
    (elif (<= (Variables|Default|GetAmountOfBlocks) 0)
      ;[1 1 1] Takes care of either going to next level or back to menu screen if its level 3
      (CallFunction|VictorySequence))))

(event EventRevertPowerups
  (bind _playerref (Variables|Default|GetPlayerRef))
  (bind _vausmesh (Variables|/Script/Arkanoid.ArkanoidPawn|GetVausMesh _playerref))
  (bind _relativescale3d (Variables|/Script/Engine.SceneComponent|GetRelativeScale3D _vausmesh))
  ;[1 1 1] Revere Power Up Effects - Made in C++ , Implemented in Blueprints
  (Transformation|SetRelativeScale3D _vausmesh (Math|Vector|MakeVector (.x _relativescale3d) (.y (Variables|/Script/Arkanoid.ArkanoidPawn|GetDefaultSize _playerref)) (.z _relativescale3d)))
  (Components|Box|SetBoxExtent (Variables|/Game/Blueprints/BP_ArkanoidPawn.BP_ArkanoidPawn_C|GetRightSide _playerref) "30.000000,38.000000,32.000000" true)
  (bind _outactors (Actor|GetAllActorsOfClass "/Script/Arkanoid.Ball"))
  (Transformation|SetWorldScale3D (Variables|/Script/Arkanoid.Ball|GetBallMesh (Utilities|Array|Get(acopy) _outactors)) "0.750000,0.750000,0.750000")
  (Variables|/Script/Arkanoid.Ball|SetSpeedMultiplier (Utilities|Array|Get(acopy) _outactors) (Variables|/Script/Arkanoid.Ball|GetDefaultSpeedMultipler (Utilities|Array|Get(acopy) _outactors)))
  (Variables|/Script/Arkanoid.ArkanoidPawn|SetbHasPowerUp (Variables|Default|GetPlayerRef) false))

(fn ConstructionScript)

(fn ResetBallandPlayer
  (Variables|Default|SetBallsInLevel 1)
  (bind _returnvalue (Game|SpawnActorfromClass "/Game/Blueprints/BP_Ball.BP_Ball_C" (Math|Transform|MakeTransform "0, 0, 0" "0, 0, 0" "1.000000,1.000000,1.000000") "Undefined" 0 0))
  (Variables|Default|SetSpawnBall _returnvalue)
  (Transformation|SetRelativeScale3D (Variables|/Script/Arkanoid.Ball|GetBallMesh _returnvalue) "0.750000,0.750000,0.750000")
  (bind _asbp_arkanoid_pawn (Utilities|Casting|CastToBP_ArkanoidPawn (Game|Player|GetPlayerPawn 0)))
  (Variables|Default|SetPlayerRef _asbp_arkanoid_pawn)
  (Transformation|AttachComponentToComponent _returnvalue (Variables|/Script/Arkanoid.ArkanoidPawn|GetVausMesh _asbp_arkanoid_pawn) "Ball" "SnapToTarget" "KeepRelative" "KeepWorld" true)
  (Variables|Default|SetBallAttached true)
  (Transformation|SetActorLocation _returnvalue (+ (Transformation|GetActorLocation _returnvalue) "0,100.000000,0.000000") false false)
  (return))

(fn VictorySequence
  (bind _returnvalue (Game|GetPlayerController 0))
  (Math|Integer|DecrementInt (Variables|/Script/Arkanoid.ArkanoidGameInstance|GetLevelsRemaining (Variables|Default|GetGameInstanceRef))
    (:%20%20
      (Game|SetGamePaused true)
      (bind _returnvalue_2 (UserInterface|CreateWidget "/Game/Blueprints/UI/Widget_VictoryScreen.Widget_VictoryScreen_C"))
      (Input|SetInputModeUIOnly _returnvalue _returnvalue_2 "DoNotLock")
      (UserInterface|Viewport|AddtoViewport _returnvalue_2 0)
      (Variables|/Script/Engine.PlayerController|SetbShowMouseCursor _returnvalue true))))