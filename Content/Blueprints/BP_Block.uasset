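; BP_Block is a block that can spawn a random power-up when its C++ code calls SpawnPowerUp.
; If CanSpawnPowerups is set, the event spawns a scaled-up BP_PowerUp offset from the block mesh at a fixed height.
; A random roll then assigns the slow, multiball or enlarge type and applies a matching colored material to the power-up mesh.
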(event EventBeginPlay)

(event Collision|EventActorBeginOverlap
  (params (OtherActor :type Actor%20Object%20Reference)))

(event EventTick
  (params (DeltaSeconds :type Float%20%28single-precision%29)))

(event EventSpawnPowerUp
  (bind _blockmesh (Variables|Default|GetBlockMesh))
  (bind _returnvalue (Transformation|GetWorldLocation _blockmesh))
  ;[1 1 1] Blueprint Impelemented and called in c++
  (if (Variables|Default|GetbCanSpawnPowerups)
    (bind _returnvalue_2 (Game|SpawnActorfromClass "/Game/Blueprints/BP_PowerUp.BP_PowerUp_C" (Math|Transform|MakeTransform (Math|Vector|MakeVector (+ (.x _returnvalue) 8e+01) (.y _returnvalue) 1.5e+02) "0, 0, 0" "1.500000,1.500000,1.500000") "Undefined" 0 0))
    (switch int (Math|Random|RandomIntegerinRange 0 2)
      (:Default
        (Variables|/Script/Arkanoid.PowerUp|SetPowerUpType _returnvalue_2 "ENLARGE" :!label _label)
        (Rendering|Material|SetMaterial (Variables|/Script/Arkanoid.PowerUp|GetPowerUpMesh _returnvalue_2) 0 "/Game/Materials/Material_Instances/MI_BlockBlue.MI_BlockBlue"))
      (:0
        (Variables|/Script/Arkanoid.PowerUp|SetPowerUpType _returnvalue_2 "SLOW")
        (Rendering|Material|SetMaterial (Variables|/Script/Arkanoid.PowerUp|GetPowerUpMesh _returnvalue_2) 0 "/Game/Materials/Material_Instances/MI_BlockOrange.MI_BlockOrange"))
      (:1
        (Variables|/Script/Arkanoid.PowerUp|SetPowerUpType _returnvalue_2 "MULTIBALL")
        (Rendering|Material|SetMaterial (Variables|/Script/Arkanoid.PowerUp|GetPowerUpMesh _returnvalue_2) 0 "/Game/Materials/Material_Instances/MI_BlockCyan.MI_BlockCyan"))
      (:2
        (goto _label)))))

(fn ConstructionScript)