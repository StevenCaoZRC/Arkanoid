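; Player paddle pawn for an Arkanoid game that launches the ball, bounces it and handles pausing.
; Space detaches the game mode's spawned ball and launches it with an impulse.
; Left and right overlap boxes zero the ball's velocity, then apply opposite 45-degree impulses instead of relying on physical bounce.
; P or Escape toggles the pause menu, and a power-up event enlarges the paddle mesh and resizes both boxes.
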(event OnComponentBeginOverlap(RightSide)
  (params (OverlappedComponent :type Primitive%20Component%20Object%20Reference) (OtherActor :type Actor%20Object%20Reference) (OtherComp :type Primitive%20Component%20Object%20Reference) (OtherBodyIndex :type Integer) (bFromSweep :type Boolean) (SweepResult :type Hit%20Result%20Structure%20%28by%20ref%29))
  ;[1 1 1] Bounce ball back to the Right in 45 degree angle
  (bind _asbp_ball (Utilities|Casting|CastToBP_Ball OtherActor))
  (Physics|SetPhysicsLinearVelocity (Variables|/Script/Arkanoid.Ball|GetBallMesh _asbp_ball) "0, 0, 0" false "None")
  (Physics|AddImpulse (Variables|/Script/Arkanoid.Ball|GetBallMesh _asbp_ball) (Math|Vector|MakeVector (* (Variables|Default|GetSpeedMultiplier) -1.0) (Variables|Default|GetSpeedMultiplier) 0.0) "None" true))

(event OnComponentBeginOverlap(LeftSide)
  (params (OverlappedComponent :type Primitive%20Component%20Object%20Reference) (OtherActor :type Actor%20Object%20Reference) (OtherComp :type Primitive%20Component%20Object%20Reference) (OtherBodyIndex :type Integer) (bFromSweep :type Boolean) (SweepResult :type Hit%20Result%20Structure%20%28by%20ref%29))
  (bind _speedmultiplier (Variables|Default|GetSpeedMultiplier))
  ;[1 1 1] Bounce ball back to the left in 45 degree angle
  (bind _asbp_ball (Utilities|Casting|CastToBP_Ball OtherActor))
  (Physics|SetPhysicsLinearVelocity (Variables|/Script/Arkanoid.Ball|GetBallMesh _asbp_ball) "0, 0, 0" false "None")
  (Physics|AddImpulse (Variables|/Script/Arkanoid.Ball|GetBallMesh _asbp_ball) (Math|Vector|MakeVector _speedmultiplier _speedmultiplier 0.0) "None" true))

(event EventSetSizeforPowerUp
  (bind _vausmesh (Variables|Default|GetVausMesh))
  ;[1 1 1] Sizing up the player when power up is enlarge
  (Transformation|SetRelativeScale3D _vausmesh (Math|Vector|MakeVector 1.0 (* (.y (Variables|/Script/Engine.SceneComponent|GetRelativeScale3D _vausmesh)) 1.5) 1.0))
  (Components|Box|SetBoxExtent (Variables|Default|GetLeftSide) "46.000000,23.000000,32.000000" true))

(event Input|KeyboardEvents|Escape
  (params (Key :type Key%20Structure :default "None"))
  ;[1 1 1] Pause Game
  (:Pressed
    (if (Variables|Default|GetIsGamePaused)
      (Game|SetGamePaused false)
      (Variables|Default|SetIsGamePaused false)
      (Widget|RemovefromParent (Variables|Default|GetWidget_InGameMenu))
      (Variables|/Script/Engine.PlayerController|SetbShowMouseCursor (Game|GetPlayerController 0) false)
      (Input|SetInputModeGameOnly (Game|GetPlayerController 0))
      (else
        (Game|SetGamePaused true)
        (Variables|Default|SetIsGamePaused true)
        (bind _returnvalue (UserInterface|CreateWidget "/Game/Blueprints/UI/Widget_InGameMenu.Widget_InGameMenu_C" (Game|GetPlayerController 0)))
        (bind _output_get (Variables|Default|SetWidget_InGameMenu _returnvalue))
        (Input|SetInputModeUIOnly (Game|GetPlayerController 0) _output_get "DoNotLock")
        (UserInterface|Viewport|AddtoViewport _output_get 0)
        (Variables|/Script/Engine.PlayerController|SetbShowMouseCursor (Game|GetPlayerController 0) true)))))

(event Input|KeyboardEvents|P
  (params (Key :type Key%20Structure :default "None"))
  ;[1 1 1] Pause Game
  ;;[1 1 1] Test Key for In Editor
  (:Pressed
    (if (Variables|Default|GetIsGamePaused)
      (Game|SetGamePaused false)
      (Variables|Default|SetIsGamePaused false)
      (Widget|RemovefromParent (Variables|Default|GetWidget_InGameMenu))
      (Variables|/Script/Engine.PlayerController|SetbShowMouseCursor (Game|GetPlayerController 0) false)
      (Input|SetInputModeGameOnly (Game|GetPlayerController 0))
      (else
        (Game|SetGamePaused true)
        (Variables|Default|SetIsGamePaused true)
        (bind _returnvalue (UserInterface|CreateWidget "/Game/Blueprints/UI/Widget_InGameMenu.Widget_InGameMenu_C" (Game|GetPlayerController 0)))
        (bind _output_get (Variables|Default|SetWidget_InGameMenu _returnvalue))
        (Input|SetInputModeUIOnly (Game|GetPlayerController 0) _output_get "DoNotLock")
        (UserInterface|Viewport|AddtoViewport _output_get 0)
        (Variables|/Script/Engine.PlayerController|SetbShowMouseCursor (Game|GetPlayerController 0) true)))))

(event Input|KeyboardEvents|SpaceBar
  (params (Key :type Key%20Structure :default "None"))
  ;[1 1 1] Launch Ball
  (:Pressed
    (bind _asbp_arkanoid_game_mode (Utilities|Casting|CastToBP_ArkanoidGameMode (Game|GetGameMode)))
    (if (Variables|/Game/Blueprints/BP_ArkanoidGameMode.BP_ArkanoidGameMode_C|GetBallAttached _asbp_arkanoid_game_mode)
      (Transformation|DetachFromActor (Variables|/Game/Blueprints/BP_ArkanoidGameMode.BP_ArkanoidGameMode_C|GetSpawnBall _asbp_arkanoid_game_mode) "KeepWorld" "KeepRelative" "KeepWorld")
      (Physics|AddImpulse (Variables|/Script/Arkanoid.Ball|GetBallMesh (Variables|/Game/Blueprints/BP_ArkanoidGameMode.BP_ArkanoidGameMode_C|GetSpawnBall _asbp_arkanoid_game_mode)) (Math|Vector|MakeVector (* (Variables|/Script/Arkanoid.Ball|GetSpeedMultiplier (Variables|/Game/Blueprints/BP_ArkanoidGameMode.BP_ArkanoidGameMode_C|GetSpawnBall _asbp_arkanoid_game_mode)) -1.0) (Variables|/Script/Arkanoid.Ball|GetSpeedMultiplier (Variables|/Game/Blueprints/BP_ArkanoidGameMode.BP_ArkanoidGameMode_C|GetSpawnBall _asbp_arkanoid_game_mode)) 0.0) "None" true)
      (Variables|/Game/Blueprints/BP_ArkanoidGameMode.BP_ArkanoidGameMode_C|SetBallAttached _asbp_arkanoid_game_mode false))))

(fn ConstructionScript)