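; BP_DeadZone is the Arkanoid kill zone that handles balls and power-ups falling into its collision component.
; An overlapping Ball decrements the game mode's BallsInLevel and is destroyed, clearing the pawn's HasPowerUp when no balls remain.
; Any other overlapping actor also clears HasPowerUp.
; For a BP_PowerUp, DestroyActor then targets the dead zone itself, not the power-up.
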(event OnComponentBeginOverlap(CollisionComponent)
  (params (OverlappedComponent :type Primitive%20Component%20Object%20Reference) (OtherActor :type Actor%20Object%20Reference) (OtherComp :type Primitive%20Component%20Object%20Reference) (OtherBodyIndex :type Integer) (bFromSweep :type Boolean) (SweepResult :type Hit%20Result%20Structure%20%28by%20ref%29))
  ;[1 1 1] Dead Zone - Destroy Ball when it falls into zone , Reset player has power up, decreased ball in game and destroys current ball
  (bind _asball (Utilities|Casting|CastToBall OtherActor)
    (:then
      (bind _asbp_arkanoid_game_mode (Utilities|Casting|CastToBP_ArkanoidGameMode (Game|GetGameMode)))
      (bind _result (Math|Integer|DecrementInt (Variables|/Script/Arkanoid.ArkanoidGameModeBase|GetBallsInLevel _asbp_arkanoid_game_mode))
        (:%20%20
          (if (<= _result 0)
            (bind _asarkanoid_pawn (Utilities|Casting|CastToArkanoidPawn (Game|Player|GetPlayerPawn 0)))
            (Variables|/Script/Arkanoid.ArkanoidPawn|SetbHasPowerUp _asarkanoid_pawn false))
          (Actor|DestroyActor _asball))))
    (:CastFailed
      (Utilities|Casting|CastToBP_PowerUp OtherActor
        (:then
          (bind _asarkanoid_pawn_2 (Utilities|Casting|CastToArkanoidPawn (Game|Player|GetPlayerPawn 0)))
          (Variables|/Script/Arkanoid.ArkanoidPawn|SetbHasPowerUp _asarkanoid_pawn_2 false)
          (Actor|DestroyActor))
        (:CastFailed
          (bind _asarkanoid_pawn_3 (Utilities|Casting|CastToArkanoidPawn (Game|Player|GetPlayerPawn 0)))
          (Variables|/Script/Arkanoid.ArkanoidPawn|SetbHasPowerUp _asarkanoid_pawn_3 false))))))

(event EventBeginPlay)

(event Collision|EventActorBeginOverlap
  (params (OtherActor :type Actor%20Object%20Reference)))

(event EventTick
  (params (DeltaSeconds :type Float%20%28single-precision%29)))

(fn ConstructionScript)