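; Power-up Blueprint for an Arkanoid-style game that implements the multi-ball effect, triggered from C++ ApplyPowerUpEffects.
; SpawnMultiBall spawns a new BP_Ball at the first ball found in the level and increments the game mode's BallsInLevel count.
; The new ball gets an impulse built from the existing ball's negated X and Y velocity, sending it the opposite way.
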(event EventBeginPlay)

(event Collision|EventActorBeginOverlap
  (params (OtherActor :type Actor%20Object%20Reference)))

(event EventTick
  (params (DeltaSeconds :type Float%20%28single-precision%29)))

(event EventSpawnMultiBall
  ;[1 1 1] Spawns another ball where the current ball is (called in c++ ApplyPowerUpEffects Powerup.cpp)
  (bind _outactors (Actor|GetAllActorsOfClass "/Game/Blueprints/BP_Ball.BP_Ball_C"))
  (Utilities|IsValid (Utilities|Array|Get(acopy) _outactors)
    (:Is%20Valid
      (bind _returnvalue (Game|SpawnActorfromClass "/Game/Blueprints/BP_Ball.BP_Ball_C" (Math|Transform|MakeTransform (Transformation|GetWorldLocation (Variables|/Script/Arkanoid.Ball|GetBallMesh (Utilities|Array|Get(acopy) _outactors)))) "Undefined" 0 0))
      (bind _asbp_arkanoid_game_mode (Utilities|Casting|CastToBP_ArkanoidGameMode (Game|GetGameMode)))
      (Math|Integer|IncrementInt (Variables|/Script/Arkanoid.ArkanoidGameModeBase|GetBallsInLevel _asbp_arkanoid_game_mode)
        (:%20%20
          (bind _returnvalue_2 (Physics|GetPhysicsLinearVelocity (Variables|/Script/Arkanoid.Ball|GetBallMesh (Utilities|Array|Get(acopy) _outactors)) "None"))
          (Physics|AddImpulse (Variables|/Script/Arkanoid.Ball|GetBallMesh _returnvalue) (Math|Vector|MakeVector (* (.x _returnvalue_2) -1.0) (* (.y _returnvalue_2) -1.0) 0.0) "None" false))))
    (:Is%20Not%20Valid
      (Development|PrintString "No balls were found in level" false))))

(fn ConstructionScript)